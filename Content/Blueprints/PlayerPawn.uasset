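; Player pawn Blueprint that sets up the local player's HUD and reads health from its HealthComp component.
; On BeginPlay, a locally controlled pawn creates the crosshair and health indicator widgets and adds both to the viewport.
; On Tick, it prints the current health on screen as a debug readout, also only when locally controlled.
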(event EventBeginPlay
  (if (Pawn|IsLocallyControlled)
    (Utilities|FlowControl|Sequence
      (:then_0
        (bind _returnvalue (UserInterface|CreateWidget "/Game/UI/WBP_Croshair.WBP_Croshair_C"))
        (UserInterface|Viewport|AddtoViewport _returnvalue 0))
      (:then_1
        (bind _returnvalue_2 (UserInterface|CreateWidget "/Game/UI/WBP_HealthIndicator.WBP_HealthIndicator_C"))
        (UserInterface|Viewport|AddtoViewport _returnvalue_2 0)))))

(event EventTick
  (params (DeltaSeconds :type Float%20%28single-precision%29))
  (if (Pawn|IsLocallyControlled)
    (Development|PrintString (Utilities|String|ToString(Float) (Variables|/Script/CoopGame.SHealthComponent|GetHealth (Variables|Default|GetHealthComp))) true true "(R=0.000000,G=0.660000,B=1.000000,A=1.000000)" 0.0)))

(fn ConstructionScript)